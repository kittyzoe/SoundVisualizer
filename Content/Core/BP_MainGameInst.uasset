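; Game instance that holds the playlist save data for the session and exposes it to the rest of the game.
; On Init it constructs a BP_PlaylistSaveCmp and caches the data its load call returns.
; Save and update events forward to that data after validity checks, while the last browsing path is read and written on it directly.
; The instance's own LoadPlaylistSaveData event only prints a debug string.
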(event EventInit
  (Utilities|FlowControl|Sequence
    (:then_0
      (bind _returnvalue (Game|ConstructObjectfromClass "/Game/Core/SaveGame/BP_PlaylistSaveCmp.BP_PlaylistSaveCmp_C"))
      (bind _playlistsavedata (Default|LoadPlaylistSaveData _returnvalue))
      (Variables|Default|SetPlaylistSaveData _playlistsavedata))))

(event EventLoadPlaylistSaveData
  (Development|PrintString "Load playlist save data  interface...."))

(event EventSavePlaylistSaveData
  (bind _playlistsavedata (Variables|Default|GetPlaylistSaveData))
  (if (Utilities|IsValid _playlistsavedata)
    (Default|SavePlaylistSaveData _playlistsavedata)))

(event EventUpdPlaylistSaveData
  (bind _playlistsavedata (Variables|Default|GetPlaylistSaveData))
  (if (Utilities|IsValid _playlistsavedata)
    (Default|UpdPlaylistSaveData _playlistsavedata)))

(event EventKeepLastBrowsingPath
  (params (NewPath :type String))
  (Variables|/Game/Core/SaveGame/BP_PlaylistSaveCmp.BP_PlaylistSaveCmp_C|SetLastBrowsingPath (Variables|Default|GetPlaylistSaveData) NewPath))

(fn FetchLastBrowsingPath
  (return (Variables|/Game/Core/SaveGame/BP_PlaylistSaveCmp.BP_PlaylistSaveCmp_C|GetLastBrowsingPath (Variables|Default|GetPlaylistSaveData))))