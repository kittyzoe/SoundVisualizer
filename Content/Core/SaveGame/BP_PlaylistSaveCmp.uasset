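; BP_PlaylistSaveCmp is a save-game object that handles loading and saving playlist data in its own named slot.
; Loading returns the saved object from that slot, or creates a fresh, unsaved instance when the slot is missing or the cast fails.
; Saving writes the object itself to the slot and prints success or failure.
; The update function is a stub that only prints a debug message.
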(fn LoadPlaylistSaveData
  (bind _returnvalue (SaveGame|DoesSaveGameExist (Variables|Default|GetPlaylistSlotName)))
  (if _returnvalue
    (bind _returnvalue_2 (SaveGame|LoadGamefromSlot (Variables|Default|GetPlaylistSlotName)))
    (bind _asbp_playlist_save_cmp (Utilities|Casting|CastToBP_PlaylistSaveCmp _returnvalue_2)
      (:then
        (return _asbp_playlist_save_cmp))
      (:CastFailed
        _)))
  (bind _sd (CallFunction|CreateEmptyPlaylistSaveData))
  (return _sd))

(fn CreateEmptyPlaylistSaveData
  (bind _returnvalue (SaveGame|CreateSaveGameObject "BP_PlaylistSaveCmp_C"))
  (return _returnvalue))

(fn UpdPlaylistSaveData
  (Development|PrintString 0 "Upd playlist....."))

(fn SavePlaylistSaveData
  (bind _returnvalue (SaveGame|SaveGametoSlot self (Variables|Default|GetPlaylistSlotName)))
  (if _returnvalue
    (Development|PrintString 0 "Save playlist done....")
    (else
      (Development|PrintString 0 "Save playlist Failed...."))))