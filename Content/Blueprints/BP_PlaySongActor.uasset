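; BP_PlaySongActor drives a music player that visualizes a song's spectrum and beats through an FMOD audio manager.
; On BeginPlay it constructs BP_FmodAudioManager, initializes linear and log spectrum bars, and shows WBP_SongPlayer, binding its play and pause events.
; Playing starts beat detection and displays the song name, or prints an error.
; While a song plays, Tick updates FMOD and pushes spectrum and beat values to the widget.
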(event Custom|PlaySongEvt
  (bind _returnvalue (Class|FmodAudioManager|PlaySong (Variables|Default|GetFmodAudio)))
  (if (> _returnvalue 0)
    (Development|PrintString (Utilities|String|Append "Play Song Error:  " (Utilities|String|ToString(Integer) _returnvalue)))
    (else
      (Variables|Default|SetIsSongPlaying true)
      (Class|FmodAudioManager|InitBeatDetector (Variables|Default|GetFmodAudio))
      (Default|UpdSongName (Variables|Default|GetSongPlayerWid) (Utilities|Text|ToText(String) (Class|FmodAudioManager|GetSongName (Variables|Default|GetFmodAudio)))))))

(event Custom|PauseSongEvt
  (params (IsPause :type Boolean))
  (Class|FmodAudioManager|PauseSong (Variables|Default|GetFmodAudio) IsPause)
  (Variables|Default|SetIsSongPlaying (not IsPause)))

(event Custom|Hzf
  (bind _songplayerwid (Variables|Default|GetSongPlayerWid))
  (bind _fmodaudio (Variables|Default|GetFmodAudio))
  (if (Variables|Default|GetIsSongPlaying)
    (Class|FmodAudioManager|UpdFmodSystem _fmodaudio)
    (bind _freqvalues (Class|FmodAudioManager|FecthLinerSpectrum _fmodaudio (Variables|Default|GetLinerBarCnt)))
    (Default|UpdLinerRTVals _songplayerwid _freqvalues)
    (bind _freqvalues_2 (Class|FmodAudioManager|FecthLogSpectrum (Variables|Default|GetFmodAudio) (Variables|Default|GetLogBarCnt)))
    (Default|UpdLogRTVals _songplayerwid _freqvalues_2)
    (bind (_freqvalues_3 _freqaveragevalues _isboss _islowm) (Class|FmodAudioManager|FecthBeat (Variables|Default|GetFmodAudio)))
    (Default|UpdRTBeatVals _songplayerwid _freqvalues_3 _freqaveragevalues _isboss _islowm)))

(event EventBeginPlay
  (Utilities|FlowControl|Sequence
    (:then_0
      (CallFunction|InitAudioManager)
      (bind _returnvalue (Class|FmodAudioManager|InitLinerSpectrum (Variables|Default|GetFmodAudio) (Variables|Default|GetBarsCount)))
      (Variables|Default|SetLinerBarCnt _returnvalue)
      (bind _returnvalue_2 (Class|FmodAudioManager|InitLogSpectrum (Variables|Default|GetFmodAudio) (Variables|Default|GetBarsCount)))
      (Variables|Default|SetLogBarCnt _returnvalue_2))
    (:then_1
      (bind _returnvalue_3 (UserInterface|CreateWidget "/Game/UI/WBP_SongPlayer.WBP_SongPlayer_C"))
      (bind _output_get (Variables|Default|SetSongPlayerWid _returnvalue_3))
      (Default|ShowMe _output_get (Variables|Default|GetLinerBarCnt) (Variables|Default|GetLogBarCnt))
      (EventDispatchers|BindEventtoDoPlaySong _output_get (delegate Custom|PlaySongEvt))
      (EventDispatchers|BindEventtoDoPauseSong _output_get (delegate Custom|PauseSongEvt)))))

(event Collision|EventActorBeginOverlap
  (params (OtherActor :type Actor%20Object%20Reference)))

(event EventTick
  (params (DeltaSeconds :type Float%20%28single-precision%29))
  (CallFunction|Hzf))

(fn ConstructionScript)

(fn InitAudioManager
  (bind _returnvalue (Game|ConstructObjectfromClass "/Game/Blueprints/BP_FmodAudioManager.BP_FmodAudioManager_C"))
  (bind _output_get (Variables|Default|SetFmodAudio _returnvalue))
  (Class|FmodAudioManager|InitializeManager _output_get))